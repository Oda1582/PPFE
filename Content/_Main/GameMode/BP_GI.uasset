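; Game instance Blueprint that persists per-level progress (the DTHS float map and unlock flags) through BP_SaveGame.
; Firsttimerunninggame builds both maps from DT_Level rows when no save exists and the first-run flag is set.
; With an existing save, it loads, adds only missing level rows and re-saves, so new levels need no save wipe.
; Wrapper events route to shared save and load functions that copy variables to and from one slot.
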(event Custom|BeginPlayLoad
  ;[1 0.5391 0] Saving Game functions
  (bind _returnvalue (SaveGame|DoesSaveGameExist (Variables|Default|GetSave%20Game%20Slot%20Name)))
  (if _returnvalue
    (CallFunction|LoadSaveGame)
    (else
      (CallFunction|SaveSaveGame))))

(event Custom|SaveGame
  ;[1 0.5391 0] Saving Game functions
  (CallFunction|SaveSaveGame))

(event Custom|LoadGame
  ;[1 0.5391 0] Saving Game functions
  (CallFunction|LoadSaveGame))

(event Custom|Save%20First%20Time%20Running
  ;[1 0.5391 0] Saving Game functions
  (bind _returnvalue (SaveGame|DoesSaveGameExist (Variables|Default|GetSave%20Game%20Slot%20Name)))
  (if _returnvalue
    (CallFunction|LoadSaveGame)
    (else
      (CallFunction|SaveSaveGame))))

(event Custom|Save%20Everything
  ;[1 0.5391 0] Saving Game functions
  (CallFunction|SaveSaveGame))

(event Custom|First%20time%20running%20game
  (bind _returnvalue (SaveGame|DoesSaveGameExist (Variables|Default|GetSave%20Game%20Slot%20Name)))
  (if _returnvalue
    ;[1 0 0.7734] Load Variables before checking the progress
    (CallFunction|BeginPlayLoad)
    ;[1 0.1406 0] Get Level info
    (bind _outrownames (DataTable|GetDataTableRowNames "/Game/_Main/Blueprints/DataTable/DT_Level.DT_Level"))
    (for _array_element _outrownames
      ;[0.4766 0 1] Checks if the Key was already added in the map variable, prevents needing to delete your save game
      (if (not (Utilities|Map|Contains (Variables|Default|GetDT_HS) (Utilities|String|ToString(Name) _array_element)))
        ;[1 0.2109 0] Adds the new levels and saves it
        (Utilities|Map|Add (Variables|Default|GetDT_HS) (Utilities|String|ToString(Name) _array_element) 0.0)
        (Utilities|Map|Add (Variables|Default|GetDT_IsLevelUnlocked) (Utilities|String|ToString(Name) _array_element) false)))
    (CallFunction|SaveSaveGame)
    ;[0.7344 0 1] Loads info again at the end just in case
    (CallFunction|BeginPlayLoad)
    (else
      ;[0.9453 1 0] Create Level Infos for the game running for the first time
      (if (Variables|Default|GetFirstTimeRunningGame)
        (bind _outrownames_2 (DataTable|GetDataTableRowNames "/Game/_Main/Blueprints/DataTable/DT_Level.DT_Level"))
        (for _array_element_2 _outrownames_2
          (Utilities|Map|Add (Variables|Default|GetDT_HS) (Utilities|String|ToString(Name) _array_element_2) 0.0)
          (Utilities|Map|Add (Variables|Default|GetDT_IsLevelUnlocked) (Utilities|String|ToString(Name) _array_element_2) false))
        (Variables|Default|SetFirstTimeRunningGame false)
        (Development|PrintString "Level Info Created" true true "(R=0.000000,G=1.000000,B=0.000000,A=1.000000)")
        (CallFunction|SaveFirstTimeRunning)))))

(fn SaveSaveGame
  (bind _returnvalue (SaveGame|DoesSaveGameExist (Variables|Default|GetSave%20Game%20Slot%20Name)))
  (if _returnvalue
    _
    (else
      (bind _returnvalue_2 (SaveGame|CreateSaveGameObject "/Game/_Main/Blueprints/Save/BP_SaveGame.BP_SaveGame_C"))
      (Variables|Default|SetAs%20BP%20Save%20Game _returnvalue_2)
      (Development|PrintString "Created Save Game" true true "(R=0.000000,G=1.000000,B=0.000000,A=1.000000)")))
  (Utilities|FlowControl|Sequence
    (:then_0
      ;[0 0.6484 1] Save Level info
      (Variables|/Game/_Main/Blueprints/Save/BP_SaveGame.BP_SaveGame_C|SetSG_FirstTimeRunningGame (Variables|Default|GetAs%20BP%20Save%20Game) (Variables|Default|GetFirstTimeRunningGame))
      (Variables|/Game/_Main/Blueprints/Save/BP_SaveGame.BP_SaveGame_C|SetSG_DT_HS (Variables|Default|GetAs%20BP%20Save%20Game) (Variables|Default|GetDT_HS))
      (Variables|/Game/_Main/Blueprints/Save/BP_SaveGame.BP_SaveGame_C|SetSG_DT_IsLevelUnlocked (Variables|Default|GetAs%20BP%20Save%20Game) (Variables|Default|GetDT_IsLevelUnlocked)))
    (:then_1
      ;[0 0.9531 1] Save files
      (SaveGame|SaveGametoSlot (Variables|Default|GetAs%20BP%20Save%20Game) (Variables|Default|GetSave%20Game%20Slot%20Name))
      (Development|PrintString "Game Saved !" true true "(R=0.000000,G=1.000000,B=0.000000,A=1.000000)"))))

(fn LoadSaveGame
  (bind _returnvalue (SaveGame|LoadGamefromSlot (Variables|Default|GetSave%20Game%20Slot%20Name)))
  (bind _asbp_save_game (Utilities|Casting|CastToBP_SaveGame _returnvalue))
  (Variables|Default|SetAs%20BP%20Save%20Game _asbp_save_game)
  (Utilities|FlowControl|Sequence
    (:then_0
      ;[1 0.7031 0] Load Level Info
      (Variables|Default|SetFirstTimeRunningGame (Variables|/Game/_Main/Blueprints/Save/BP_SaveGame.BP_SaveGame_C|GetSG_FirstTimeRunningGame (Variables|Default|GetAs%20BP%20Save%20Game)))
      (Variables|Default|SetDT_HS (Variables|/Game/_Main/Blueprints/Save/BP_SaveGame.BP_SaveGame_C|GetSG_DT_HS (Variables|Default|GetAs%20BP%20Save%20Game)))
      (Variables|Default|SetDT_IsLevelUnlocked (Variables|/Game/_Main/Blueprints/Save/BP_SaveGame.BP_SaveGame_C|GetSG_DT_IsLevelUnlocked (Variables|Default|GetAs%20BP%20Save%20Game))))
    (:then_1
      (Development|PrintString "Loaded Save Game !" true true "(R=0.008321,G=0.000000,B=1.000000,A=1.000000)"))))