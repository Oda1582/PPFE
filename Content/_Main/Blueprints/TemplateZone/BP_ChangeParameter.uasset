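; BP_ChangeParameter is a trigger box that cycles one VR pawn setting, chosen by Selection: locomotion, rotation or belt rotation type.
; Each VRPawn overlap steps through that setting's array with wraparound, prints the value, then teleports the pawn to the Bp_RespawnPoint after a short delay.
; A text label, set on BeginPlay and after each teleport, shows the current value and turns every tick to face the pawn's camera.
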(event OnComponentBeginOverlap(Box)
  (params (OverlappedComponent :type Primitive%20Component%20Object%20Reference) (OtherActor :type Actor%20Object%20Reference) (OtherComp :type Primitive%20Component%20Object%20Reference) (OtherBodyIndex :type Integer) (bFromSweep :type Boolean) (SweepResult :type Hit%20Result%20Structure%20%28by%20ref%29))
  (Utilities|Casting|CastToVRPawn OtherActor)
  (switch string (Variables|Default|GetSelection)
    (:LocomotionType
      (if (== (Variables|Default|GetCurrentParameterIndex) (- (Utilities|Array|Length (Variables|Default|GetLocomotionType)) 1))
        (Variables|/Game/VRTemplate/Blueprints/VRPawn.VRPawn_C|SetLocomotionType (Variables|Default|GetAs%20VRPawn) (Utilities|Array|Get(acopy) (Variables|Default|GetLocomotionType)))
        (Variables|Default|SetCurrentParameterIndex 0)
        (else
          (bind _result (Math|Integer|IncrementInt (Variables|Default|GetCurrentParameterIndex))
            (:%20%20
              (Variables|/Game/VRTemplate/Blueprints/VRPawn.VRPawn_C|SetLocomotionType (Variables|Default|GetAs%20VRPawn) (Utilities|Array|Get(acopy) (Variables|Default|GetLocomotionType) _result))))))
      (Development|PrintString (Utilities|String|EnumtoString (Variables|/Game/VRTemplate/Blueprints/VRPawn.VRPawn_C|GetLocomotionType (Variables|Default|GetAs%20VRPawn)))))
    (:RotationType
      (if (== (Variables|Default|GetCurrentParameterIndex) (- (Utilities|Array|Length (Variables|Default|GetRotationType)) 1))
        (Variables|/Game/VRTemplate/Blueprints/VRPawn.VRPawn_C|SetRotationType (Variables|Default|GetAs%20VRPawn) (Utilities|Array|Get(acopy) (Variables|Default|GetRotationType)))
        (Variables|Default|SetCurrentParameterIndex 0)
        (else
          (bind _result_2 (Math|Integer|IncrementInt (Variables|Default|GetCurrentParameterIndex))
            (:%20%20
              (Variables|/Game/VRTemplate/Blueprints/VRPawn.VRPawn_C|SetRotationType (Variables|Default|GetAs%20VRPawn) (Utilities|Array|Get(acopy) (Variables|Default|GetRotationType) _result_2))))))
      (Development|PrintString (Utilities|String|ToString(Byte) (Variables|/Game/VRTemplate/Blueprints/VRPawn.VRPawn_C|GetRotationType (Variables|Default|GetAs%20VRPawn)))))
    (:BeltRotationType
      (if (== (Variables|Default|GetCurrentParameterIndex) (- (Utilities|Array|Length (Variables|Default|GetBeltRotationType)) 1))
        (Variables|/Game/VRTemplate/Blueprints/VRPawn.VRPawn_C|SetBeltRotationType (Variables|Default|GetAs%20VRPawn) (Utilities|Array|Get(acopy) (Variables|Default|GetBeltRotationType)))
        (Variables|Default|SetCurrentParameterIndex 0)
        (else
          (bind _result_3 (Math|Integer|IncrementInt (Variables|Default|GetCurrentParameterIndex))
            (:%20%20
              (Variables|/Game/VRTemplate/Blueprints/VRPawn.VRPawn_C|SetBeltRotationType (Variables|Default|GetAs%20VRPawn) (Utilities|Array|Get(acopy) (Variables|Default|GetBeltRotationType) _result_3))))))
      (Development|PrintString (Utilities|String|ToString(Byte) (Variables|/Game/VRTemplate/Blueprints/VRPawn.VRPawn_C|GetBeltRotationType (Variables|Default|GetAs%20VRPawn))))))
  (Utilities|FlowControl|Delay 0.1)
  (Transformation|SetActorLocation (Variables|Default|GetAs%20VRPawn) (Transformation|GetWorldLocation (Variables|/Game/_Main/Blueprints/TemplateZone/Bp_RespawnPoint.Bp_RespawnPoint_C|GetDefaultSceneRoot (Variables|Default|GetRespawnRef))) false true)
  (switch string (Variables|Default|GetSelection)
    (:LocomotionType
      (Rendering|Components|TextRender|SetText (Variables|Default|GetTextRender) (Utilities|Text|ToText(String) (Utilities|String|EnumtoString (Variables|/Game/VRTemplate/Blueprints/VRPawn.VRPawn_C|GetLocomotionType (Variables|Default|GetAs%20VRPawn))))))
    (:RotationType
      (Rendering|Components|TextRender|SetText (Variables|Default|GetTextRender) (Utilities|Text|ToText(String) (Utilities|String|EnumtoString (Variables|/Game/VRTemplate/Blueprints/VRPawn.VRPawn_C|GetRotationType (Variables|Default|GetAs%20VRPawn))))))
    (:BeltRotationType
      (Rendering|Components|TextRender|SetText (Variables|Default|GetTextRender) (Utilities|Text|ToText(String) (Utilities|String|EnumtoString (Variables|/Game/VRTemplate/Blueprints/VRPawn.VRPawn_C|GetBeltRotationType (Variables|Default|GetAs%20VRPawn))))))))

(event EventBeginPlay
  (bind _asvrpawn (Utilities|Casting|CastToVRPawn (Game|GetPlayerCharacter 0)))
  (Variables|Default|SetAs%20VRPawn _asvrpawn)
  (bind _returnvalue (Actor|GetActorOfClass "/Game/_Main/Blueprints/TemplateZone/Bp_RespawnPoint.Bp_RespawnPoint_C"))
  (Variables|Default|SetRespawnRef _returnvalue)
  (switch string (Variables|Default|GetSelection)
    (:LocomotionType
      (Rendering|Components|TextRender|SetText (Variables|Default|GetTextRender) (Utilities|Text|ToText(String) (Utilities|String|EnumtoString (Variables|/Game/VRTemplate/Blueprints/VRPawn.VRPawn_C|GetLocomotionType (Variables|Default|GetAs%20VRPawn))))))
    (:RotationType
      (Rendering|Components|TextRender|SetText (Variables|Default|GetTextRender) (Utilities|Text|ToText(String) (Utilities|String|EnumtoString (Variables|/Game/VRTemplate/Blueprints/VRPawn.VRPawn_C|GetRotationType (Variables|Default|GetAs%20VRPawn))))))
    (:BeltRotationType
      (Rendering|Components|TextRender|SetText (Variables|Default|GetTextRender) (Utilities|Text|ToText(String) (Utilities|String|EnumtoString (Variables|/Game/VRTemplate/Blueprints/VRPawn.VRPawn_C|GetBeltRotationType (Variables|Default|GetAs%20VRPawn))))))))

(event Collision|EventActorBeginOverlap
  (params (OtherActor :type Actor%20Object%20Reference)))

(event EventTick
  (params (DeltaSeconds :type Float%20%28single-precision%29))
  (Transformation|SetWorldRotation (Variables|Default|GetTextRender) (Math|Rotator|FindLookatRotation (Transformation|GetWorldLocation (Variables|Default|GetTextRender)) (Transformation|GetWorldLocation (Variables|/Game/VRTemplate/Blueprints/VRPawn.VRPawn_C|GetCamera (Variables|Default|GetAs%20VRPawn)))) false false))

(fn ConstructionScript)