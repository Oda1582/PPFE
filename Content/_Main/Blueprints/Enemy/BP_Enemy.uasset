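; VR enemy that spots and faces the player, takes per-bone bullet damage and ragdolls on death.
; Detection sphere overlap runs a line trace to set detection, a second sphere clears it, and Tick yaws the capsule toward the pawn.
; BulletDamage scales head, limb (bone mass) or seeded body damage.
; Non-hip hits timeline-blend physics below the bone with an impulse, while death enables full physics and notifies VRGameMode.
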(event OnComponentBeginOverlap(DetectionSphere)
  (params (OverlappedComponent :type Primitive%20Component%20Object%20Reference) (OtherActor :type Actor%20Object%20Reference) (OtherComp :type Primitive%20Component%20Object%20Reference) (OtherBodyIndex :type Integer) (bFromSweep :type Boolean) (SweepResult :type Hit%20Result%20Structure%20%28by%20ref%29))
  (bind _asvrpawn (Utilities|Casting|CastToVRPawn OtherActor))
  (Variables|Default|SetAs%20VRPawn _asvrpawn)
  (bind _returnvalue (Collision|LineTraceByChannel (Transformation|GetWorldLocation (Variables|Default|GetArrow1)) (Transformation|GetWorldLocation (Variables|/Script/Engine.Character|GetCapsuleComponent _asvrpawn)) "TraceTypeQuery2" false 0 "Persistent"))
  (if _returnvalue
    (Development|PrintString "see me ")
    (Variables|Default|SetPlayerDetected true)
    (else
      (Development|PrintString "doesn't see me ")
      (Variables|Default|SetPlayerDetected false))))

(event OnComponentEndOverlap(DetectionSphere)
  (params (OverlappedComponent :type Primitive%20Component%20Object%20Reference) (OtherActor :type Actor%20Object%20Reference) (OtherComp :type Primitive%20Component%20Object%20Reference) (OtherBodyIndex :type Integer)))

(event OnComponentEndOverlap(LoseDetectionSphere)
  (params (OverlappedComponent :type Primitive%20Component%20Object%20Reference) (OtherActor :type Actor%20Object%20Reference) (OtherComp :type Primitive%20Component%20Object%20Reference) (OtherBodyIndex :type Integer))
  (Utilities|Casting|CastToVRPawn OtherActor)
  (Development|PrintString "doesn't see me ")
  (Variables|Default|SetPlayerDetected false))

(event EventBeginPlay)

(event Collision|EventActorBeginOverlap
  (params (OtherActor :type Actor%20Object%20Reference)))

(event EventTick
  (params (DeltaSeconds :type Float%20%28single-precision%29))
  (Utilities|FlowControl|Sequence
    (:then_0
      (if (and (> (Variables|Default|GetBlendWeight) 0.0) (not (Variables|Default|GetIsDead)))
        (Class|SkeletalMeshComponent|SetAllBodiesBelowSimulatePhysics (Variables|Character|GetMesh) (Variables|Default|GetBone) true true)
        (Class|SkeletalMeshComponent|SetAllBodiesBelowPhysicsBlendWeight (Variables|Character|GetMesh) (Variables|Default|GetBone) (Variables|Default|GetBlendWeight) false true)
        (elif (Variables|Default|GetIsDead)
          (Class|SkeletalMeshComponent|SetAllBodiesSimulatePhysics (Variables|Character|GetMesh) true))))
    (:then_1
      (if (and (Variables|Default|GetPlayerDetected) (not (Variables|Default|GetIsDead)))
        (Transformation|SetWorldRotation (Variables|Collision|GetCapsuleComponent) (Math|Rotator|MakeRotator 0.0 0.0 (.yaw (Math|Rotator|FindLookatRotation (Transformation|GetWorldLocation (Variables|Default|GetGun)) (Transformation|GetWorldLocation (Variables|/Script/Engine.Character|GetCapsuleComponent (Variables|Default|GetAs%20VRPawn)))))) false false)))))

(event EventBulletDamage
  (params (Damage%20Seed :type Integer) (Bone :type Name :default "None") (Impulse :type Vector :default "0, 0, 0") (Damage%20Multiplier :type Float%20%28double-precision%29) (Instigator :type Pawn%20Object%20Reference))
  (bind _mesh (Variables|Character|GetMesh))
  ;[1 0 0.4219] Check not dead
  (if (and (not (Variables|Default|GetIsDead)) (!= Bone ""))
    ;[0.9219 1 0] Return damage depending on the body part
    (bind _damage (CallFunction|ReturnDamageBasedonBoneHit Bone Damage%20Multiplier Damage%20Seed))
    (bind _output_get (Variables|Default|SetHealth (- (Variables|Default|GetHealth) _damage)))
    (Variables|Default|SetBone Bone)
    (Variables|Default|SetImpulse Impulse)
    (Development|PrintText (Utilities|Text|FormatText "Health : {hl} 
Damage : {dmg}" _output_get _damage))
    (if (> (Variables|Default|GetHealth) 0.0)
      (|ValidBoneHit
        (:True
          (Utilities|FlowControl|Sequence
            (:then_0
              (bind _blendalpha (Timeline|Blend PlayFromStart)
                (:Update
                  (Variables|Default|SetBlendWeight _blendalpha))
                (:Finished
                  (Class|SkeletalMeshComponent|SetAllBodiesPhysicsBlendWeight _mesh 0.0 false)
                  (Class|SkeletalMeshComponent|SetAllBodiesSimulatePhysics _mesh false)
                  (Variables|Default|SetPhysicsBlend false))))
            (:then_1
              (Utilities|FlowControl|Delay 0.05)
              (Physics|AddImpulse (Variables|Character|GetMesh) (Variables|Default|GetImpulse) (Variables|Default|GetBone) true)))))
      (else
        (Variables|Default|SetBlendWeight 0.0)
        (Variables|Default|SetHealth 0.0)
        (if (!= (Variables|Default|GetBone) "Hips")
          (Class|SkeletalMeshComponent|SetAllBodiesSimulatePhysics (Variables|Character|GetMesh) true)
          (Physics|AddImpulse (Variables|Character|GetMesh) (* (Variables|Default|GetImpulse) 0.3) (Variables|Default|GetBone) true)
          (else
            (Class|SkeletalMeshComponent|SetAllBodiesSimulatePhysics (Variables|Character|GetMesh) true)))
        (Variables|Default|SetIsDead true)
        (Collision|SetCollisionResponsetoChannel (Variables|Collision|GetCapsuleComponent) "ECC_Pawn" "ECR_Ignore")
        (bind _asvrgame_mode (Utilities|Casting|CastToVRGameMode (Game|GetGameMode)))
        (Default|NotifyEnemyDeath _asvrgame_mode)))))

(fn ConstructionScript)

(fn ReturnDamageBasedonBoneHit
  (params (Bone :type Name) (DamageMultiplier :type Float%20%28double-precision%29) (Seed :type Integer))
  (bind _returnvalue (Math|Random|MakeRandomStream Seed))
  (LocalVariables|SetHit%20Bone Bone)
  (LocalVariables|SetDamage%20Multiplier DamageMultiplier)
  (LocalVariables|SetHeadShotDamage (Math|Random|RandomFloatinRangefromStream _returnvalue 1e+02 1e+02))
  (LocalVariables|SetBodyDamage (Math|Random|RandomFloatinRangefromStream _returnvalue 1e+01 5e+01))
  (return (* DamageMultiplier (Math|Float|SelectFloat (LocalVariables|GetHeadShotDamage) (Math|Float|SelectFloat (Class|SkeletalMeshComponent|GetBoneMass (Variables|Character|GetMesh) (LocalVariables|GetHit%20Bone) true) (LocalVariables|GetBodyDamage) (CallFunction|LimpHit? (LocalVariables|GetHit%20Bone))) (CallFunction|HeadHit? (LocalVariables|GetHit%20Bone))))))

(fn LimpHit?
  (params (HitBone :type Name))
  (return (Math|Boolean|ORBoolean (or (Class|SkinnedMeshComponent|BoneIsChildOf (Variables|Character|GetMesh) HitBone "LeftArm") (== HitBone "LeftArm")) (or (Class|SkinnedMeshComponent|BoneIsChildOf (Variables|Character|GetMesh) HitBone "RightArm") (== HitBone "RightArm")) (or (Class|SkinnedMeshComponent|BoneIsChildOf (Variables|Character|GetMesh) HitBone "LeftUpLeg") (== HitBone "LeftUpLeg")) (or (Class|SkinnedMeshComponent|BoneIsChildOf (Variables|Character|GetMesh) HitBone "RightUpLeg") (== HitBone "RightUpLeg")))))

(fn HeadHit?
  (params (HitBone :type Name))
  (return (or (Class|SkinnedMeshComponent|BoneIsChildOf (Variables|Character|GetMesh) HitBone "Neck") (== HitBone "Neck"))))