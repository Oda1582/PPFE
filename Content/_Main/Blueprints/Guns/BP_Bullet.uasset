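; Bullet projectile actor that resolves its impact when its sphere component hits something, then destroys itself.
; A hit prints the actor name, attaches a fading decal, and spawns particles and sound through surface-type selects that currently share the same assets.
; BPI_Damage actors receive a random damage seed, bone, impulse and multiplier, with player pawn 0 as instigator.
; Other physics-simulating components just get an impulse along the impact normal.
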(event OnComponentHit(Sphere)
  (params (HitComponent :type Primitive%20Component%20Object%20Reference) (OtherActor :type Actor%20Object%20Reference) (OtherComp :type Primitive%20Component%20Object%20Reference) (NormalImpulse :type Vector :default "0, 0, 0") (Hit :type Hit%20Result%20Structure%20%28by%20ref%29))
  (Development|PrintText (Utilities|Text|FormatText "Actor : {actor} " OtherActor))
  (CallFunction|ImpactDecals Hit)
  (bind _randomseed (CallFunction|RandomDamageSeed))
  (CallFunction|ImpactSound Hit)
  (CallFunction|ApplyPhysicsandDamage _randomseed Hit)
  (Actor|DestroyActor))

(event OnComponentBeginOverlap(Sphere)
  (params (OverlappedComponent :type Primitive%20Component%20Object%20Reference) (OtherActor :type Actor%20Object%20Reference) (OtherComp :type Primitive%20Component%20Object%20Reference) (OtherBodyIndex :type Integer) (bFromSweep :type Boolean) (SweepResult :type Hit%20Result%20Structure%20%28by%20ref%29)))

(event EventBeginPlay
  (Components|StaticMesh|SetStaticMesh (Variables|Default|GetBullet) (Variables|Default|GetBulletMesh)))

(event Collision|EventActorBeginOverlap
  (params (OtherActor :type Actor%20Object%20Reference)))

(event EventTick
  (params (DeltaSeconds :type Float%20%28single-precision%29)))

(fn ConstructionScript)

(fn ImpactDecals
  (params (Hit :type Hit%20Result%20Structure))
  (bind (_bblockinghit _binitialoverlap _time _distance _location _impactpoint _normal _impactnormal _physmat _hitactor _hitcomponent) (Collision|BreakHitResult Hit))
  (Utilities|IsValid _physmat
    (:Is%20Valid
      (switch Utilities|FlowControl|Switch|SwitchonEPhysicalSurface (Variables|/Script/PhysicsCore.PhysicalMaterial|GetSurfaceType _physmat)
        (:SurfaceType_Default
          (CallFunction|BulletDefaultHitDecal _hitcomponent _impactpoint _normal)
          (return))))
    (:Is%20Not%20Valid
      (return))))

(fn RandomDamageSeed
  (return (Math|Random|RandomIntegerinRange 0 100)))

(fn ImpactSound
  (params (Hit :type Hit%20Result%20Structure))
  (bind (_bblockinghit _binitialoverlap _time _distance _location _impactpoint _normal _impactnormal _physmat) (Collision|BreakHitResult Hit))
  (bind _surfacetype (Variables|/Script/PhysicsCore.PhysicalMaterial|GetSurfaceType _physmat))
  (if _bblockinghit
    (Niagara|SpawnSystematLocation (Utilities|Select :Index _surfacetype :SurfaceType_Default "/Game/_Main/NS/Handgun/P_BulletImpact_default.P_BulletImpact_default" :SurfaceType1 "/Game/_Main/NS/Handgun/P_BulletImpact_default.P_BulletImpact_default" :SurfaceType2 "/Game/_Main/NS/Handgun/P_BulletImpact_default.P_BulletImpact_default" :SurfaceType3 "/Game/_Main/NS/Handgun/P_BulletImpact_default.P_BulletImpact_default" :SurfaceType4 "/Game/_Main/NS/Handgun/P_BulletImpact_default.P_BulletImpact_default") _impactpoint (Math|Conversions|RotationFromXVector _impactnormal))
    (Audio|SpawnSoundatLocation (Utilities|Select :Index _surfacetype :SurfaceType_Default "/Game/_Main/Asset/Guns/Global/Audio/BulletImpactConcrete_Cue.BulletImpactConcrete_Cue" :SurfaceType1 "/Game/_Main/Asset/Guns/Global/Audio/BulletImpactConcrete_Cue.BulletImpactConcrete_Cue" :SurfaceType2 "/Game/_Main/Asset/Guns/Global/Audio/BulletImpactConcrete_Cue.BulletImpactConcrete_Cue" :SurfaceType3 "/Game/_Main/Asset/Guns/Global/Audio/BulletImpactConcrete_Cue.BulletImpactConcrete_Cue" :SurfaceType4 "/Game/_Main/Asset/Guns/Global/Audio/BulletImpactConcrete_Cue.BulletImpactConcrete_Cue") _impactpoint "0, 0, 0" 2.0 1.0 0.0 "/Game/_Main/Asset/Guns/Global/Audio/BulletImpactAttenuation.BulletImpactAttenuation" 0)))

(fn ApplyPhysicsandDamage
  (params (Seed :type Integer) (Hit :type Hit%20Result%20Structure))
  (bind (_bblockinghit _binitialoverlap _time _distance _location _impactpoint _normal _impactnormal _physmat _hitactor _hitcomponent _hitbonename) (Collision|BreakHitResult Hit))
  (Variables|Default|SetDamade%20Seed Seed)
  (if _bblockinghit
    (if (Utilities|DoesObjectImplementInterface _hitactor "/Game/_Main/Blueprints/Interface/BPI_Damage.BPI_Damage_C")
      ;[0.5703 1 0] Damage
      (Class|BPIDamage|BulletDamage(Message) _hitactor (Variables|Default|GetDamade%20Seed) _hitbonename (* _impactnormal (/ (Variables|Default|GetImpactForce) 2.0)) (Variables|Default|GetDamage%20Multiplier) (Game|Player|GetPlayerPawn 0))
      (return)
      (elif (Physics|IsSimulatingPhysics _hitcomponent "None")
        (Physics|AddImpulse _hitcomponent (* _impactnormal (/ (Variables|Default|GetImpactForce) 2.0)) "None" false)
        (return)))))

(fn BulletDefaultHitDecal
  (params (Hit%20Component :type Primitive%20Component%20Object%20Reference) (Hit%20Location :type Vector) (Normal :type Vector))
  (bind _returnvalue (Class|GameplayStatics|SpawnDecalAttached (Variables|Default|GetImpactDecalVFX) "2.000000,2.000000,2.000000" Hit%20Component "None" Hit%20Location (Math|Conversions|RotationFromXVector Normal) "KeepWorldPosition" 1e+01))
  (Utilities|IsValid _returnvalue
    (:Is%20Valid
      (Rendering|Components|Decal|SetFadeScreenSize _returnvalue 0.001)
      (Rendering|Components|Decal|SetFadeIn _returnvalue 0.0 0.01)
      (Rendering|Components|Decal|SetFadeOut _returnvalue 15.0 15.0 false))))