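; VR gun actor with grab-based handling: hand-specific input contexts, analog trigger, firing-mode switching and magazine release.
; The grabbed slide follows the motion controller on a clamped axis via looping timers, ejecting and chambering rounds with sound and haptics.
; Overlapping a held, matching magazine releases it and eases it into its socket.
; Only semi-automatic fire is handled, consuming rounds or playing empty sounds; trace, decal and recoil helpers are never called.
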(event EventBeginPlay
  (if (not (CallFunction|HasFiringModes))
    (Development|PrintString "NO FIRING MODE ADDED TO THE GUN" true true "(R=1.000000,G=0.000000,B=0.000000,A=1.000000)")))

(event Collision|EventActorBeginOverlap
  (params (OtherActor :type Actor%20Object%20Reference)))

(event EventTick
  (params (DeltaSeconds :type Float%20%28single-precision%29)))

(event OnGrabbed(MainGrabComponent)
  (params (MotionController :type Motion%20Controller%20Component%20Object%20Reference))
  ;[0 1 0.0625] Main Grab
  (Variables|Default|GetMotion%20Controller
    (:then
      (|RemoveMappingfromOppositeHand))
    (:else
      _))
  (Variables|Default|SetMotion%20Controller MotionController)
  (bind _holding_hand_anim (CallFunction|GetHoldingHandAnim))
  (Variables|Default|SetHolding%20Hand%20Anim _holding_hand_anim)
  (Input|EnableInput (Game|GetPlayerController 0))
  (Input|AddMappingContext (PlayerController|LocalPlayerSubsystems|GetEnhancedInputLocalPlayerSubsystem (Game|GetPlayerController 0)) (select (Utilities|Enum|Equal(Enum) (Default|GetHeldbyHand (Variables|Default|GetMainGrabComponent)) "Left") "/Game/VRTemplate/Input/IMC_Weapon_Left.IMC_Weapon_Left" "/Game/VRTemplate/Input/IMC_Weapon_Right.IMC_Weapon_Right") 1 "(bIgnoreAllPressedKeysUntilRelease=True,bForceImmediately=False,bNotifyUserSettings=False)"))

(event OnDropped(MainGrabComponent)
  ;[0 1 0.0625] Main Grab
  (Input|DisableInput (Game|GetPlayerController 0) 0)
  (Input|RemoveMappingContext (PlayerController|LocalPlayerSubsystems|GetEnhancedInputLocalPlayerSubsystem (Game|GetPlayerController 0)) (select (Utilities|Enum|Equal(Enum) (Default|GetHeldbyHand (Variables|Default|GetMainGrabComponent)) "Left") "/Game/VRTemplate/Input/IMC_Weapon_Left.IMC_Weapon_Left" "/Game/VRTemplate/Input/IMC_Weapon_Right.IMC_Weapon_Right") "(bIgnoreAllPressedKeysUntilRelease=True,bForceImmediately=False,bNotifyUserSettings=False)"))

(event Input|EnhancedActionEvents|EnhancedInputActionIA_GunShoot_Left
  (params (ActionValue :type Float%20%28double-precision%29) (ElapsedSeconds :type Float%20%28double-precision%29) (TriggeredSeconds :type Float%20%28double-precision%29) (InputAction :type Input%20Action%20Object%20Reference :default "/Game/VRTemplate/Input/Actions/IA_GunShoot_Left.IA_GunShoot_Left"))
  (:Triggered
    (|LeftHandFireTrigger ActionValue :!label _label
      (:Trigger%20Passed%20Threshold
        (if (CallFunction|HasFiringModes)
          (switch Utilities|FlowControl|Switch|SwitchonENUM_FiringModes (Variables|Default|GetCurrentFiringMode)
            (:NewEnumerator1
              (if (not (Variables|Default|GetTriggerPressed))
                (Variables|Default|SetTriggerPressed true)
                (CallFunction|SingleShot))))))
      (:Trigger%20has%20not%20Passed%20Threshold
        (Variables|Default|SetTriggerPressed false))))
  (:Canceled
    (goto _label Trigger%20is%20not%20Pressed%20/%20Canceled))
  (:Completed
    (goto _label Trigger%20is%20not%20Pressed%20/%20Canceled)))

(event Input|EnhancedActionEvents|EnhancedInputActionIA_GunShoot_Right
  (params (ActionValue :type Float%20%28double-precision%29) (ElapsedSeconds :type Float%20%28double-precision%29) (TriggeredSeconds :type Float%20%28double-precision%29) (InputAction :type Input%20Action%20Object%20Reference :default "/Game/VRTemplate/Input/Actions/IA_GunShoot_Right.IA_GunShoot_Right"))
  (:Triggered
    (|RightHandFireTrigger ActionValue :!label _label
      (:Trigger%20Passed%20Threshold
        (if (CallFunction|HasFiringModes)
          (switch Utilities|FlowControl|Switch|SwitchonENUM_FiringModes (Variables|Default|GetCurrentFiringMode)
            (:NewEnumerator1
              (if (not (Variables|Default|GetTriggerPressed))
                (Variables|Default|SetTriggerPressed true)
                (CallFunction|SingleShot))))))
      (:Trigger%20has%20not%20Passed%20Threshold
        (Variables|Default|SetTriggerPressed false))))
  (:Canceled
    (goto _label Trigger%20is%20not%20pressed%20/%20Canceled))
  (:Completed
    (goto _label Trigger%20is%20not%20pressed%20/%20Canceled)))

(event OnGrabbed(CurlGrabComponent)
  (params (MotionController :type Motion%20Controller%20Component%20Object%20Reference))
  ;[0.8281 1 0 1 50] Grabbing Slide
  (CallFunction|AttachHandtoSlide MotionController)
  ;;[1 0 0.5625] Play Slider Grabbed Sound
  (Audio|PlaySoundatLocation (Variables|Default|GetSlideGrabbedSoundCue) (Transformation|GetWorldLocation (Variables|Default|GetSlideGrabCollision)) "0, 0, 0" 1.0 1.0 0.0 0 0 0 0)
  ;;[0.8984 0 1] Set Initial Offset for handles
  (Variables|Default|SetInitial%20Grab%20Offset (CallFunction|GetGrabbedOffsetBetweenMC&Slide))
  (Variables|Default|SetSliderReleased false)
  ;;[1 0.5391 0] Timer for moving the slider while grabbed
  (Utilities|Time|SetTimerbyEvent (delegate Custom|Interpolate%20Slide%20Movement) 0.01 true))

(event OnDropped(CurlGrabComponent)
  ;[1 0.1406 0 1 50] Releasing Slide
  (CallFunction|DetachHandfromSlide)
  ;;[1 0.4219 0] Clearing References
  (Variables|Default|SetSlide%20Grab%20Motion%20Controller 0)
  (Variables|Default|SetSlide%20Motion%20Controller%20HandMesh 0)
  (Class|KismetSystemLibrary|PauseTimer 0 "Interpolate Slide Movement")
  (if (<= (Variables|Default|GetCurrentSlideOffset) (Variables|Default|GetOffsetToPlayReleaseSound))
    ;;[0 0.7891 1] Play Released Sound FX
    (Audio|PlaySoundatLocation (Variables|Default|GetSlideReleasedSoundCue) (Transformation|GetWorldLocation (Variables|Default|GetMuzzle)) "0, 0, 0" 1.0 1.0 0.0 0 0 0 0)
    (CallFunction|PlayHapticEffectonOppositeHand 1.0))
  (Variables|Default|SetSliderReleased true)
  (Utilities|Time|SetTimerbyEvent (delegate Custom|ReturnSlideBack) 0.01 true))

(event Custom|Interpolate%20Slide%20Movement
  (bind _charginghandlemaxdistance (Variables|Default|GetChargingHandleMaxDistance))
  (bind _returnvalue (CallFunction|ClampSlideMovement _charginghandlemaxdistance))
  ;[0.8281 1 0 1 50] Grabbing Slide
  ;;[0 0.5547 1] Current position of handle
  (Variables|Default|SetCurrentSlideOffset _returnvalue)
  (if (and (== _returnvalue (Variables|Default|GetChargingHandleMaxDistance)) (not (Variables|Default|GetReachedLockPosition)))
    ;;[1 0 0.2812] Play Cocking Sound
    (Variables|Default|SetReachedLockPosition true)
    (Audio|PlaySoundatLocation (Variables|Default|GetHandgunCockSoundCue) (Transformation|GetWorldLocation (Variables|Default|GetSlideGrabCollision)) "0, 0, 0" 1.0 1.0 0.0 0 0 0 0)
    ;;[0 0.5781 1] Gun Communication Logic
    (bind _magazine (Variables|Default|GetMagazine)
      (:then
        (if (Variables|/Game/_Main/Blueprints/Guns/BP_Magazine.BP_Magazine_C|GetIsEmpty _magazine)
          (Variables|Default|SetDryFire true :!label _label)
          (Variables|Default|SetBullet%20Is%20Ready%20to%20be%20taken%20from%20Mag false)
          (else
            (Variables|Default|SetDryFire false)
            (Variables|Default|SetBullet%20Is%20Ready%20to%20be%20taken%20from%20Mag true))))
      (:else
        (goto _label)))
    (if (Variables|Default|GetChamber%20Has%20Bullet)
      (CallFunction|InitiateBulletThrowandSetRoundMeshInvinsible))
    (CallFunction|PlayHapticEffect 0.8)
    (elif (Variables|Default|GetReachedLockPosition)
      (if (>= (Variables|Default|GetCurrentSlideOffset) (+ (Variables|Default|GetChargingHandleMaxDistance) (Variables|Default|GetDistanceToTravelBackFromLockToGetBullet)))
        (bind _magazine_2 (Variables|Default|GetMagazine)
          (:then
            (if (Variables|/Game/_Main/Blueprints/Guns/BP_Magazine.BP_Magazine_C|GetIsEmpty _magazine_2)
              (Rendering|SetVisibility (Variables|Default|GetRound) false false)
              (Variables|Default|SetChamber%20Has%20Bullet false)
              (else
                (Rendering|SetVisibility (Variables|Default|GetRound) true false)
                (Default|RemoveRound _magazine_2)
                (Variables|Default|SetChamber%20Has%20Bullet true)))
            (Variables|Default|SetReachedLockPosition false))
          (:else
            _)))))
  ;;[1 0 0.9844] Assigning Current Slide position to handle
  (Transformation|SetRelativeLocation (Variables|Default|GetHandle) (Math|Vector|MakeVector (Variables|Default|GetCurrentSlideOffset) 0.0 0.0) false false))

(event Custom|ReturnSlideBack
  ;[1 0.1406 0 1 50] Releasing Slide
  ;;[0 1 0.1094] Move Handle back to its original position
  (bind _hasreachedorigin (CallFunction|InterpolateHandletoInitialPositionandContinueOnceDone))
  (if _hasreachedorigin
    ;;[1 0 0.5625] Stop the function to move to original position
    (Transformation|SetRelativeLocation (Variables|Default|GetHandle) (Math|Vector|MakeVector 0.0 0.0 0.0) false false)
    (Class|KismetSystemLibrary|PauseTimer 0 "ReturnSlideBack")
    (Variables|Default|SetCurrentSlideOffset 0.0)
    (if (Variables|Default|GetReachedLockPosition)
      (bind _magazine (Variables|Default|GetMagazine)
        (:then
          (if (Variables|Default|GetBullet%20Is%20Ready%20to%20be%20taken%20from%20Mag)
            (if (Variables|/Game/_Main/Blueprints/Guns/BP_Magazine.BP_Magazine_C|GetIsEmpty _magazine)
              (if (Variables|Default|GetChamber%20Has%20Bullet)
                (Variables|Default|SetDryFire true :!label _label)
                (Rendering|SetVisibility (Variables|Default|GetRound) false false)
                (Variables|Default|SetChamber%20Has%20Bullet false)
                (Variables|Default|SetReachedLockPosition false :!label _label_2))
              (else
                (Default|RemoveRound (Variables|Default|GetMagazine))
                (Rendering|SetVisibility (Variables|Default|GetRound) true false)
                (Variables|Default|SetChamber%20Has%20Bullet true)
                (goto _label_2)))
            (else
              (Variables|Default|SetReachedLockPosition false :!label _label_3)
              (goto _label))))
        (:else
          (goto _label_3))))))

(event OnComponentBeginOverlap(MagazineCollision)
  (params (OverlappedComponent :type Primitive%20Component%20Object%20Reference) (OtherActor :type Actor%20Object%20Reference) (OtherComp :type Primitive%20Component%20Object%20Reference) (OtherBodyIndex :type Integer) (bFromSweep :type Boolean) (SweepResult :type Hit%20Result%20Structure%20%28by%20ref%29))
  ;[1 0 0.5859 1 72] Inserting Magazine
  ;;[0 0.2969 1] Check if we don't have a magazine and if we overlap one
  (Variables|Default|GetMagazine
    (:then)
    (:else
      (bind _asbp_magazine (Utilities|Casting|CastToBP_Magazine OtherActor))
      ;;[0.2188 0 1] Check that it's held and for the right type of gun
      (if (Utilities|Enum|Equal(Enum) (Variables|Default|GetGunType) (Variables|/Game/_Main/Blueprints/Guns/BP_Magazine.BP_Magazine_C|GetMagazineType _asbp_magazine))
        (if (Variables|/Game/VRTemplate/Blueprints/CurlGrabComponent.CurlGrabComponent_C|GetbIsHeld (Variables|/Game/_Main/Blueprints/Guns/BP_Magazine.BP_Magazine_C|GetCurlGrabComponent _asbp_magazine))
          ;;[1 0.7969 0] Deactivate physics
          (bind _output_get (Variables|Default|SetMagazine _asbp_magazine))
          (Physics|SetSimulatePhysics (Variables|/Game/_Main/Blueprints/Guns/BP_Magazine.BP_Magazine_C|GetMagazineMesh _output_get) false)
          (Variables|/Game/VRTemplate/Blueprints/CurlGrabComponent.CurlGrabComponent_C|SetbSimulateOnDrop (Variables|/Game/_Main/Blueprints/Guns/BP_Magazine.BP_Magazine_C|GetCurlGrabComponent _output_get) false)
          ;;[0 0.2266 1] Play a sound and drop the magazine from the hand
          (Default|PlayIn/outSound (Variables|Default|GetMagazine) true)
          (Default|TryRelease (Variables|/Game/_Main/Blueprints/Guns/BP_Magazine.BP_Magazine_C|GetCurlGrabComponent (Variables|Default|GetMagazine)))
          (EventDispatchers|BindEventtoOnGrabbed (Variables|/Game/_Main/Blueprints/Guns/BP_Magazine.BP_Magazine_C|GetCurlGrabComponent (Variables|Default|GetMagazine)) (delegate Custom|Simulate%20Magazine%20Physics%20%20On%20Dropped))
          (Utilities|Time|SetTimerbyEvent (delegate Custom|Smooth%20Attachment) 0.01 true))))))

(event Custom|Simulate%20Magazine%20Physics%20%20On%20Dropped
  (params (MotionController :type Motion%20Controller%20Component%20Object%20Reference))
  ;[1 0 0.5859 1 72] Inserting Magazine
  ;;[0.1016 0 1] Prevent from having physics when trying to grab it again
  (Variables|/Game/VRTemplate/Blueprints/CurlGrabComponent.CurlGrabComponent_C|SetbSimulateOnDrop (Variables|/Game/_Main/Blueprints/Guns/BP_Magazine.BP_Magazine_C|GetCurlGrabComponent (Variables|Default|GetMagazine)) true)
  (EventDispatchers|UnbindEventfromOnGrabbed (Variables|/Game/_Main/Blueprints/Guns/BP_Magazine.BP_Magazine_C|GetCurlGrabComponent (Variables|Default|GetMagazine)) (delegate Custom|Simulate%20Magazine%20Physics%20%20On%20Dropped))
  (Variables|Default|SetMagazine 0))

(event Custom|Smooth%20Attachment
  ;[1 0 0.5859 1 72] Inserting Magazine
  ;;[0.875 0 1] Interpolate the Magazine to be inserted smoothly
  (bind _returnvalue (CallFunction|SmoothMagazineAttachmentandContinueOnceDone))
  (if _returnvalue
    (Transformation|AttachComponentToComponent (Variables|Default|GetMagazine) (Variables|Default|GetGunMesh) "Magazine" "SnapToTarget" "SnapToTarget" "KeepRelative" true)
    (Class|KismetSystemLibrary|PauseTimer 0 "Smooth Attachment")))

(event Input|EnhancedActionEvents|EnhancedInputActionIA_SwitchGunMode_Left
  (params (ActionValue :type Boolean) (ElapsedSeconds :type Float%20%28double-precision%29) (TriggeredSeconds :type Float%20%28double-precision%29) (InputAction :type Input%20Action%20Object%20Reference :default "/Game/VRTemplate/Input/Actions/IA_SwitchGunMode_Left.IA_SwitchGunMode_Left"))
  (:Completed
    (CallFunction|SwitchGunMode)))

(event Input|EnhancedActionEvents|EnhancedInputActionIA_SwitchGunMode_Right
  (params (ActionValue :type Boolean) (ElapsedSeconds :type Float%20%28double-precision%29) (TriggeredSeconds :type Float%20%28double-precision%29) (InputAction :type Input%20Action%20Object%20Reference :default "/Game/VRTemplate/Input/Actions/IA_SwitchGunMode_Right.IA_SwitchGunMode_Right"))
  (:Completed
    (CallFunction|SwitchGunMode)))

(event Input|EnhancedActionEvents|EnhancedInputActionIA_DropMagLeft
  (params (ActionValue :type Boolean) (ElapsedSeconds :type Float%20%28double-precision%29) (TriggeredSeconds :type Float%20%28double-precision%29) (InputAction :type Input%20Action%20Object%20Reference :default "/Game/VRTemplate/Input/Actions/IA_DropMagLeft.IA_DropMagLeft"))
  (:Completed
    (bind _magazine (Variables|Default|GetMagazine)
      (:then
        (Default|PlayIn/outSound _magazine false)
        (Transformation|DetachFromComponent (Variables|/Game/_Main/Blueprints/Guns/BP_Magazine.BP_Magazine_C|GetMagazineMesh _magazine) "KeepWorld" "KeepWorld" "KeepWorld" true)
        (Physics|SetSimulatePhysics (Variables|/Game/_Main/Blueprints/Guns/BP_Magazine.BP_Magazine_C|GetMagazineMesh _magazine) true)
        (EventDispatchers|UnbindallEventsfromOnGrabbed (Variables|/Game/_Main/Blueprints/Guns/BP_Magazine.BP_Magazine_C|GetCurlGrabComponent (Variables|Default|GetMagazine)))
        (Variables|/Game/VRTemplate/Blueprints/CurlGrabComponent.CurlGrabComponent_C|SetbSimulateOnDrop (Variables|/Game/_Main/Blueprints/Guns/BP_Magazine.BP_Magazine_C|GetCurlGrabComponent (Variables|Default|GetMagazine)) true)
        (Variables|Default|SetMagazine 0))
      (:else))))

(event Input|EnhancedActionEvents|EnhancedInputActionIA_DropMagRight
  (params (ActionValue :type Boolean) (ElapsedSeconds :type Float%20%28double-precision%29) (TriggeredSeconds :type Float%20%28double-precision%29) (InputAction :type Input%20Action%20Object%20Reference :default "/Game/VRTemplate/Input/Actions/IA_DropMagRight.IA_DropMagRight"))
  (:Completed
    (bind _magazine (Variables|Default|GetMagazine)
      (:then
        (Default|PlayIn/outSound _magazine false)
        (Transformation|DetachFromComponent (Variables|/Game/_Main/Blueprints/Guns/BP_Magazine.BP_Magazine_C|GetMagazineMesh _magazine) "KeepWorld" "KeepWorld" "KeepWorld" true)
        (Physics|SetSimulatePhysics (Variables|/Game/_Main/Blueprints/Guns/BP_Magazine.BP_Magazine_C|GetMagazineMesh _magazine) true)
        (EventDispatchers|UnbindallEventsfromOnGrabbed (Variables|/Game/_Main/Blueprints/Guns/BP_Magazine.BP_Magazine_C|GetCurlGrabComponent (Variables|Default|GetMagazine)))
        (Variables|/Game/VRTemplate/Blueprints/CurlGrabComponent.CurlGrabComponent_C|SetbSimulateOnDrop (Variables|/Game/_Main/Blueprints/Guns/BP_Magazine.BP_Magazine_C|GetCurlGrabComponent (Variables|Default|GetMagazine)) true)
        (Variables|Default|SetMagazine 0))
      (:else))))

(fn ConstructionScript)

(fn GetHoldingHandAnim
  (bind _maingrabcomponent (Variables|Default|GetMainGrabComponent))
  (if (Utilities|Enum|Equal(Enum) (Default|GetHeldbyHand _maingrabcomponent) "Left")
    (return (Variables|/Game/VRTemplate/Blueprints/GrabComponent.GrabComponent_C|GetLeft%20Hand%20Anim _maingrabcomponent))
    (else
      (return (Variables|/Game/VRTemplate/Blueprints/GrabComponent.GrabComponent_C|GetRight%20Hand%20Anim _maingrabcomponent)))))

(fn AttachHandtoSlide
  (params (MotionController :type Motion%20Controller%20Component%20Object%20Reference))
  (bind _output_get (Variables|Default|SetSlide%20Grab%20Motion%20Controller MotionController))
  (bind _array_element (Utilities|Array|ForEachLoopwithBreak (Components|GetChildrenComponents _output_get false) :!label _label)
    (:LoopBody
      (bind _asb_mannequins_xr (Utilities|Casting|CastToB_MannequinsXR _array_element))
      (bind _output_get_2 (Variables|Default|SetSlide%20Motion%20Controller%20HandMesh _asb_mannequins_xr))
      (Variables|Default|SetHand%20Mesh%20Relative%20Transform (Transformation|GetRelativeTransform _output_get_2))
      (goto _label Break))
    (:Completed
      (if (Utilities|Enum|Equal(Enum) (Default|GetHeldbyHand (Variables|Default|GetCurlGrabComponent)) "Right")
        (Transformation|AttachComponentToComponent _output_get_2 (Variables|Default|GetSlideHand_R) "None" "SnapToTarget" "SnapToTarget" "SnapToTarget" true)
        (else
          (Transformation|AttachComponentToComponent _output_get_2 (Variables|Default|GetSlideHand_L) "None" "SnapToTarget" "SnapToTarget" "SnapToTarget" true)))
      (return))))

(fn DetachHandfromSlide
  (bind _hand_mesh_relative_transform (Variables|Default|GetHand%20Mesh%20Relative%20Transform))
  (bind _slide_motion_controller_handmesh (Variables|Default|GetSlide%20Motion%20Controller%20HandMesh))
  (Transformation|AttachComponentToComponent (Variables|Default|GetSlide%20Motion%20Controller%20HandMesh) (Variables|Default|GetSlide%20Grab%20Motion%20Controller) "None" "SnapToTarget" "SnapToTarget" "SnapToTarget" true)
  (if (Utilities|Enum|Equal(Enum) (Default|GetHeldbyHand (Variables|Default|GetCurlGrabComponent)) "Right")
    (Transformation|AddRelativeRotation (Variables|Default|GetSlide%20Motion%20Controller%20HandMesh) (.rotation _hand_mesh_relative_transform) false false)
    (else
      (Transformation|AddRelativeRotation _slide_motion_controller_handmesh (.rotation _hand_mesh_relative_transform) false false)
      (Transformation|SetRelativeScale3D _slide_motion_controller_handmesh (.scale _hand_mesh_relative_transform))))
  (Transformation|AddRelativeLocation (Variables|Default|GetSlide%20Motion%20Controller%20HandMesh) (.location _hand_mesh_relative_transform) false false)
  (return))

(fn GetGrabbedOffsetBetweenMC&Slide
  (return (- (Transformation|GetWorldLocation (Variables|/Game/VRTemplate/Blueprints/CurlGrabComponent.CurlGrabComponent_C|GetMotionControllerRef (Variables|Default|GetCurlGrabComponent))) (Transformation|GetWorldLocation (Variables|Default|GetHandle)))))

(fn ClampSlideMovement
  (params (Min :type Float%20%28double-precision%29))
  (return (Math|Float|Clamp(Float) (+ (.x (Math|Transform|InverseTransformLocation (Transformation|GetWorldTransform (Variables|Default|GetHandle)) (- (Transformation|GetWorldLocation (Variables|/Game/VRTemplate/Blueprints/CurlGrabComponent.CurlGrabComponent_C|GetMotionControllerRef (Variables|Default|GetCurlGrabComponent))) (Variables|Default|GetInitial%20Grab%20Offset)))) (.x (Variables|/Script/Engine.SceneComponent|GetRelativeLocation (Variables|Default|GetHandle)))) Min 0.0)))

(fn InterpolateHandletoInitialPositionandContinueOnceDone
  (bind _returnvalue (Utilities|Time|GetWorldDeltaSeconds))
  (bind _handle (Variables|Default|GetHandle))
  (bind _slidersnaptooriginspeedmultiplier (Variables|Default|GetSliderSnapToOriginSpeedMultiplier))
  (bind _returnvalue_2 (* _returnvalue _slidersnaptooriginspeedmultiplier))
  (bind _relativelocation (Variables|/Script/Engine.SceneComponent|GetRelativeLocation _handle))
  (bind _returnvalue_3 (Math|Interpolation|FInterpTo (.x _relativelocation) 0.0 _returnvalue_2 0.4))
  (Transformation|SetRelativeLocation _handle (Math|Vector|MakeVector _returnvalue_3 0.0 0.0) false false)
  (return (Math|Float|NearlyEqual(Float) _returnvalue_3 0.0 0.01)))

(fn SmoothMagazineAttachmentandContinueOnceDone
  (bind _returnvalue (Utilities|Time|GetWorldDeltaSeconds))
  (bind _magazine (Variables|Default|GetMagazine))
  (bind _gunmesh (Variables|Default|GetGunMesh))
  (bind _magazinesnaptooriginspeedmultiplier (Variables|Default|GetMagazineSnapToOriginSpeedMultiplier))
  (bind _returnvalue_2 (Transformation|GetSocketLocation _gunmesh "Magazine"))
  (bind _returnvalue_3 (* _returnvalue _magazinesnaptooriginspeedmultiplier))
  (bind _magazinemesh (Variables|/Game/_Main/Blueprints/Guns/BP_Magazine.BP_Magazine_C|GetMagazineMesh _magazine))
  (bind _returnvalue_4 (Transformation|GetWorldLocation _magazinemesh))
  (bind _returnvalue_5 (Math|Interpolation|VInterpTo _returnvalue_4 _returnvalue_2 _returnvalue_3 1.0))
  (Transformation|SetRelativeLocation (Variables|/Script/Engine.Actor|GetRootComponent _magazine) _returnvalue_5 false false)
  (return (Utilities|Operators|EqualEqual _returnvalue_2 _returnvalue_5 0.01)))

(fn InitiateBulletThrowandSetRoundMeshInvinsible
  (bind _round (Variables|Default|GetRound))
  (bind _returnvalue (Transformation|GetWorldTransform _round))
  (Niagara|SpawnSystematLocation (Variables|Default|GetSlideRoundEjection) (.location _returnvalue) (.rotation _returnvalue) (.scale _returnvalue))
  (Rendering|SetVisibility (Variables|Default|GetRound) false false)
  (return))

(fn PlayHapticEffect
  (params (Scale :type Float%20%28double-precision%29))
  (Class|PlayerController|PlayHapticEffect (Game|GetPlayerController 0) (Variables|Default|GetHapticEffect) (Default|GetHeldbyHand (Variables|Default|GetCurlGrabComponent)) Scale false)
  (return))

(fn PlayHapticEffectonOppositeHand
  (params (Scale :type Float%20%28double-precision%29))
  (Class|PlayerController|PlayHapticEffect (Game|GetPlayerController 0) (Variables|Default|GetHapticEffect) (select (Utilities|Enum|Equal(Enum) (Default|GetHeldbyHand (Variables|Default|GetCurlGrabComponent)) "Left") "Right" "Left") Scale false)
  (return))

(fn SwitchGunMode
  (if (CallFunction|HasFiringModes)
    (if (== (Variables|Default|GetCurrentFiringModeIndex) (- (Utilities|Array|Length (Variables|Default|GetFiringModesAvailableForGun)) 1))
      (Variables|Default|SetCurrentFiringMode (Utilities|Array|Get(acopy) (Variables|Default|GetFiringModesAvailableForGun)))
      (Variables|Default|SetCurrentFiringModeIndex 0)
      (else
        (bind _result (Math|Integer|IncrementInt (Variables|Default|GetCurrentFiringModeIndex))
          (:%20%20
            (bind _output_get (Variables|Default|SetCurrentFiringModeIndex _result))
            (Variables|Default|SetCurrentFiringMode (Utilities|Array|Get(acopy) (Variables|Default|GetFiringModesAvailableForGun) _output_get))))))
    (Development|PrintString (Utilities|String|EnumtoString (Variables|Default|GetCurrentFiringMode)))
    (else
      (Development|PrintString "Doesn't have any firing mode assigned" true true "(R=1.000000,G=0.000000,B=0.000000,A=1.000000)"))))

(fn HasFiringModes
  (return (> (Utilities|Array|Length (Variables|Default|GetFiringModesAvailableForGun)) 0)))

(fn SingleShot
  (bind _sliderreleased (Variables|Default|GetSliderReleased))
  (Variables|Default|GetMagazine
    (:then
      (if (Variables|Default|GetChamber%20Has%20Bullet)
        (if (Variables|/Game/_Main/Blueprints/Guns/BP_Magazine.BP_Magazine_C|GetIsEmpty (Variables|Default|GetMagazine))
          (if (not _sliderreleased)
            (|DryFire/EmptyTriggerSound :!label _label))
          (elif _sliderreleased
            (Default|RemoveRound (Variables|Default|GetMagazine))
            (else
              (goto _label))))
        (else
          (goto _label))))
    (:else
      (if (not (Variables|Default|GetChamber%20Has%20Bullet))
        (goto _label)))))

(fn LineTrace,ImpactDecals&RandomizingRecoil
  (bind (_location _direction) (CallFunction|GunBarrelLocationandDirection 0.0))
  (bind _outhit (CallFunction|LineTracefromBarrel _location _direction))
  (CallFunction|ImpactDecals _outhit)
  (CallFunction|RandomizeRecoil)
  (CallFunction|RandomDamageSeed))

(fn LineTracefromBarrel
  (params (Start :type Vector) (End :type Vector))
  (bind _outhit (Collision|LineTraceByChannel Start End "TraceTypeQuery1" false 0 "None"))
  (return _outhit))

(fn GunBarrelLocationandDirection
  (params (Distance :type Float%20%28double-precision%29))
  (bind _gunmesh (Variables|Default|GetGunMesh))
  (bind _silencerattached (Variables|Default|GetSilencerAttached))
  (bind _returnvalue (Transformation|GetSocketLocation _gunmesh "Barrel"))
  (bind _returnvalue_2 (Transformation|GetSocketLocation _gunmesh "SilencerBarrel"))
  (bind _returnvalue_3 (Math|Vector|SelectVector _returnvalue_2 _returnvalue _silencerattached))
  (return _returnvalue_3 (+ _returnvalue_3 (* (Math|Vector|GetForwardVector (Transformation|GetSocketRotation _gunmesh "Barrel")) Distance))))

(fn ImpactDecals
  (params (Hit :type Hit%20Result%20Structure))
  (bind (_bblockinghit _binitialoverlap _time _distance _location _impactpoint _normal _impactnormal _physmat _hitactor _hitcomponent) (Collision|BreakHitResult Hit))
  (switch Utilities|FlowControl|Switch|SwitchonEPhysicalSurface (Variables|/Script/PhysicsCore.PhysicalMaterial|GetSurfaceType _physmat)
    (:SurfaceType_Default
      (CallFunction|BulletDefaultHitDecal _hitcomponent _impactpoint _normal))))

(fn BulletDefaultHitDecal
  (params (Hit%20Component :type Primitive%20Component%20Object%20Reference) (Hit%20Location :type Vector) (Normal :type Vector))
  (bind _returnvalue (Class|GameplayStatics|SpawnDecalAttached "/Game/_Main/Asset/Guns/Global/Materials/M_Bullet_decal.M_Bullet_decal" "2.000000,2.000000,2.000000" Hit%20Component "None" Hit%20Location (Math|Conversions|RotationFromXVector Normal) "KeepRelativeOffset" 1e+01))
  (Utilities|IsValid _returnvalue
    (:Is%20Valid
      (Rendering|Components|Decal|SetFadeScreenSize _returnvalue 0.001)
      (Rendering|Components|Decal|SetFadeIn _returnvalue 0.0 0.01)
      (Rendering|Components|Decal|SetFadeOut _returnvalue 15.0 15.0 false))))

(fn RandomizeRecoil
  ;[0 1 0.3672] Extreme Values if Gun is only Grabbed By One Hand (Recoil is Less Stable)
  (Variables|Default|SetRandomRecoilY (Math|Random|RandomFloatinRange -0.65 0.65))
  (Variables|Default|SetRandomRecoilZ (Math|Random|RandomFloatinRange 0.0 0.75)))

(fn RandomDamageSeed
  (return (Math|Random|RandomIntegerinRange 0 100)))

(fn ImpactSound
  (params (Hit :type Hit%20Result%20Structure))
  (bind (_bblockinghit _binitialoverlap _time _distance _location _impactpoint _normal _impactnormal _physmat) (Collision|BreakHitResult Hit))
  (if _bblockinghit
    (switch Utilities|FlowControl|Switch|SwitchonEPhysicalSurface (Variables|/Script/PhysicsCore.PhysicalMaterial|GetSurfaceType _physmat))))