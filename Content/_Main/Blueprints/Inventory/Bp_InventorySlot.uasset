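; VR inventory slot that holds one grabbable actor dropped inside it.
; Overlapping actors have their GrabComponents bound to grab and drop events, and the cell mesh shrinks while the slot is empty.
; On drop, the slot disables physics, attaches and shrinks the actor, optionally snapping rotation.
; Grabbing it or pulling it out detaches it and restores its scale; debug prints and unreachable older logic remain.
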(event OnComponentBeginOverlap(CellCollision)
  (params (OverlappedComponent :type Primitive%20Component%20Object%20Reference) (OtherActor :type Actor%20Object%20Reference) (OtherComp :type Primitive%20Component%20Object%20Reference) (OtherBodyIndex :type Integer) (bFromSweep :type Boolean) (SweepResult :type Hit%20Result%20Structure%20%28by%20ref%29))
  (for _array_element (Actor|GetComponentsByClass OtherActor "/Game/VRTemplate/Blueprints/GrabComponent.GrabComponent_C")
    (Utilities|Array|Add (Variables|Default|GetTrackedGrabComponents) _array_element)
    (EventDispatchers|AssignOnGrabbed _array_element (delegate Custom|OnGrabbed_Event))
    (EventDispatchers|AssignOnDropped _array_element (delegate Custom|OnDropped_Event)))
  (if (> (Utilities|Array|Length (Variables|Default|GetTrackedGrabComponents)) 0)
    (CallFunction|Increase/DecreaseCellSize false)
    (Development|PrintString "Try Decrease")
    (else
      (Development|PrintString "Won't Decrease"))))

(event OnComponentEndOverlap(CellCollision)
  (params (OverlappedComponent :type Primitive%20Component%20Object%20Reference) (OtherActor :type Actor%20Object%20Reference) (OtherComp :type Primitive%20Component%20Object%20Reference) (OtherBodyIndex :type Integer))
  (if (== OtherActor (Variables|Default|GetHeldActor))
    (for _array_element (Actor|GetComponentsByClass OtherActor "/Game/VRTemplate/Blueprints/GrabComponent.GrabComponent_C")
      (if (Variables|/Game/VRTemplate/Blueprints/GrabComponent.GrabComponent_C|GetbIsHeld _array_element)
        (Variables|Default|SetCanDrop (Variables|/Game/VRTemplate/Blueprints/GrabComponent.GrabComponent_C|GetbIsHeld _array_element))
        (Utilities|Array|RemoveItem (Variables|Default|GetTrackedGrabComponents) _array_element)
        (EventDispatchers|UnbindEventfromOnGrabbed _array_element (delegate Custom|OnGrabbed_Event))
        (EventDispatchers|UnbindEventfromOnDropped _array_element (delegate Custom|OnDropped_Event))))
    (if (Variables|Default|GetCanDrop)
      (CallFunction|TryDropObject OtherActor)
      (CallFunction|Increase/DecreaseCellSize true)
      (Variables|Default|SetCanDrop false))
    (else
      (CallFunction|TryDropObject OtherActor)
      (for _array_element_2 (Actor|GetComponentsByClass OtherActor "/Game/VRTemplate/Blueprints/GrabComponent.GrabComponent_C")
        (Utilities|Array|RemoveItem (Variables|Default|GetTrackedGrabComponents) _array_element_2)
        (EventDispatchers|UnbindEventfromOnGrabbed _array_element_2 (delegate Custom|OnGrabbed_Event))
        (EventDispatchers|UnbindEventfromOnDropped _array_element_2 (delegate Custom|OnDropped_Event)))
      (CallFunction|Increase/DecreaseCellSize true))))

(event Custom|OnGrabbed_Event
  (params (MotionController :type Motion%20Controller%20Component%20Object%20Reference) (SelfReference :type Grab%20Component%20Object%20Reference))
  (bind _returnvalue (Components|GetOwner SelfReference))
  (Development|PrintText (Utilities|Text|FormatText "Owner : {owner}" _returnvalue))
  (CallFunction|TryDropObject _returnvalue))

(event Custom|OnDropped_Event
  (params (SelfReference :type Grab%20Component%20Object%20Reference))
  (CallFunction|TryCaptureObject SelfReference)
  (CallFunction|Increase/DecreaseCellSize true))

(event EventBeginPlay
  (Variables|Default|SetInitital%20Cell%20Scale (Transformation|GetWorldScale (Variables|Default|GetCellMesh))))

(event Collision|EventActorBeginOverlap
  (params (OtherActor :type Actor%20Object%20Reference)))

(event EventTick
  (params (DeltaSeconds :type Float%20%28single-precision%29)))

(fn ConstructionScript)

(fn TryDropObject
  (params (Actor :type Actor%20Object%20Reference))
  ;[1 0 0.2344] Check it's valid and the same actor in the slot
  (Utilities|IsValid (Variables|Default|GetHeldActor)
    (:Is%20Valid
      (if (== Actor (Variables|Default|GetHeldActor))
        ;[0 0.2734 1] Check if it's indeed attached to the slot
        (if (== (Actor|GetAttachParentActor (Variables|Default|GetHeldActor)) self)
          (Transformation|DetachFromActor (Variables|Default|GetHeldActor) "KeepWorld" "KeepWorld" "KeepWorld")
          (else
            (Development|PrintString "WUHERFOUISFJK")))
        (Transformation|SetActorScale3D Actor (Variables|Default|GetInitital%20Actor%20Scale))
        (Development|PrintText (Utilities|Text|FormatText "{Actor} is Detached" (Variables|Default|GetHeldActor)))
        (Variables|Default|SetHeldActor 0)))))

(fn TryCaptureObject
  (params (GrabComponent :type Grab%20Component%20Object%20Reference))
  (Utilities|IsValid (Variables|Default|GetHeldActor)
    (:Is%20Not%20Valid
      (bind _output_get (Variables|Default|SetHeldActor (Components|GetOwner GrabComponent)))
      (Variables|Default|SetInitital%20Actor%20Scale (Transformation|GetActorScale3D _output_get))
      (Default|SetPrimitiveCompPhysics GrabComponent false)
      (Transformation|AttachComponentToComponent _output_get (Variables|Default|GetDefaultSceneRoot) "None" "SnapToTarget" "KeepWorld" "KeepWorld" true)
      (Transformation|SetActorScale3D (Variables|Default|GetHeldActor) (* (Variables|Default|GetInitital%20Actor%20Scale) (Variables|Default|GetShrinkMultiplier)))
      (Development|PrintText (Utilities|Text|FormatText "{Actor} is Attached" (Variables|Default|GetHeldActor)))
      (if (Variables|Default|GetSnapRotation)
        (Transformation|SetActorRotation (Variables|Default|GetHeldActor) (Transformation|GetWorldRotation (Variables|Default|GetRotationSnap)))))))

(fn Increase/DecreaseCellSize
  (params (Increase? :type Boolean))
  (Utilities|IsValid (Variables|Default|GetHeldActor)
    (:Is%20Not%20Valid
      (Transformation|SetWorldScale3D (Variables|Default|GetCellMesh) (select Increase? (Variables|Default|GetInitital%20Cell%20Scale) (* (Variables|Default|GetInitital%20Cell%20Scale) (Variables|Default|GetDecreaseMeshScaleMultiplier)))))))