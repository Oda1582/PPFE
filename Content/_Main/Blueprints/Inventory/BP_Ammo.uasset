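; BP_Ammo is a grabbable VR ammo pickup that refills the player's ammo reserves.
; When grabbed by a VRPawn, it adds AmmoAmount to common ammo for handgun and SMG magazine types, or to heavy ammo for rifle, sniper and shotgun types.
; It updates the pawn's ammo widget, plays a sound, forces the hand to release it, and destroys itself after a short delay unless flagged otherwise.
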(event OnGrabbed(GrabComponent)
  (params (MotionController :type Motion%20Controller%20Component%20Object%20Reference) (SelfReference :type Grab%20Component%20Object%20Reference))
  (bind _asvrpawn (Utilities|Casting|CastToVRPawn (Components|GetOwner MotionController)))
  (Variables|Default|SetAs%20VRPawn _asvrpawn)
  (switch Utilities|FlowControl|Switch|SwitchonENUM_GunType (Variables|Default|GetMagazineType)
    (:NewEnumerator0
      (bind _output_get (Variables|/Game/VRTemplate/Blueprints/VRPawn.VRPawn_C|SetCommonAmmo (Variables|Default|GetAs%20VRPawn) (+ (Variables|/Game/VRTemplate/Blueprints/VRPawn.VRPawn_C|GetCommonAmmo (Variables|Default|GetAs%20VRPawn)) (Variables|Default|GetAmmoAmount)) :!label _label))
      (Default|SetCommonAmmoTxt (Variables|/Game/VRTemplate/Blueprints/VRPawn.VRPawn_C|GetAs%20WBP%20Ammo%20Info (Variables|Default|GetAs%20VRPawn)) _output_get))
    (:NewEnumerator1
      (bind _output_get_2 (Variables|/Game/VRTemplate/Blueprints/VRPawn.VRPawn_C|SetHeavyWeaponAmmo (Variables|Default|GetAs%20VRPawn) (+ (Variables|/Game/VRTemplate/Blueprints/VRPawn.VRPawn_C|GetHeavyWeaponAmmo (Variables|Default|GetAs%20VRPawn)) (Variables|Default|GetAmmoAmount)) :!label _label_2))
      (Default|SetHeavyAmmoTxt (Variables|/Game/VRTemplate/Blueprints/VRPawn.VRPawn_C|GetAs%20WBP%20Ammo%20Info (Variables|Default|GetAs%20VRPawn)) _output_get_2))
    (:NewEnumerator2
      (goto _label_2))
    (:NewEnumerator3
      (goto _label_2))
    (:NewEnumerator4
      (goto _label)))
  (Audio|PlaySoundatLocation (Variables|Default|GetGrabAmmoSoundCue) (Transformation|GetWorldLocation (Variables|Default|GetAmmoMesh)) "0, 0, 0" 1.0 1.0 0.0 0 0 0 0)
  (Default|TryReleasingObject (Variables|Default|GetAs%20VRPawn) (Utilities|Enum|Equal(Enum) (Default|GetHeldbyHand (Variables|Default|GetGrabComponent)) "Right"))
  (if (not (Variables|Default|GetShouldn'tBeDestroyed))
    (Utilities|FlowControl|Delay 0.1)
    (Actor|DestroyActor)))

(event EventBeginPlay)

(event Collision|EventActorBeginOverlap
  (params (OtherActor :type Actor%20Object%20Reference)))

(event EventTick
  (params (DeltaSeconds :type Float%20%28single-precision%29)))

(fn ConstructionScript)