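; VR inventory belt actor that hands the player a pistol magazine when its grab component is grabbed.
; If neither hand holds anything and CommonAmmo remains, it spawns a BP_Magazine at the controller, caps its rounds to that ammo and force-grabs it into the grabbing hand.
; With an item held, it checks the other hand's gun type but does nothing further; per-type magazine spawning is unconnected, and ammo overlap events are empty.
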(event OnComponentBeginOverlap(AmmoCollision)
  (params (OverlappedComponent :type Primitive%20Component%20Object%20Reference) (OtherActor :type Actor%20Object%20Reference) (OtherComp :type Primitive%20Component%20Object%20Reference) (OtherBodyIndex :type Integer) (bFromSweep :type Boolean) (SweepResult :type Hit%20Result%20Structure%20%28by%20ref%29)))

(event OnComponentEndOverlap(AmmoCollision)
  (params (OverlappedComponent :type Primitive%20Component%20Object%20Reference) (OtherActor :type Actor%20Object%20Reference) (OtherComp :type Primitive%20Component%20Object%20Reference) (OtherBodyIndex :type Integer)))

(event OnGrabbed(GrabComponent)
  (params (MotionController :type Motion%20Controller%20Component%20Object%20Reference) (SelfReference :type Grab%20Component%20Object%20Reference))
  (bind _as_vrpawn (Variables|Default|GetAs%20VRPawn))
  (bind _as_vrpawn_2 (Variables|Default|GetAs%20VRPawn))
  (bind _as_vrpawn_3 (Variables|Default|GetAs%20VRPawn))
  (bind _commonammo (Variables|/Game/VRTemplate/Blueprints/VRPawn.VRPawn_C|GetCommonAmmo _as_vrpawn_2))
  (if (or (Utilities|IsValid (Variables|/Game/VRTemplate/Blueprints/VRPawn.VRPawn_C|GetHeldComponentLeft _as_vrpawn)) (Utilities|IsValid (Variables|/Game/VRTemplate/Blueprints/VRPawn.VRPawn_C|GetHeldComponentRight _as_vrpawn)))
    (bind _asbp_gun (Utilities|Casting|CastToBP_Gun (Components|GetOwner (select (Utilities|Enum|Equal(Enum) (Default|GetHeldbyHand (Variables|Default|GetGrabComponent)) "Left") (Variables|/Game/VRTemplate/Blueprints/VRPawn.VRPawn_C|GetHeldComponentRight _as_vrpawn_3) (Variables|/Game/VRTemplate/Blueprints/VRPawn.VRPawn_C|GetHeldComponentLeft _as_vrpawn_3)))))
    (switch Utilities|FlowControl|Switch|SwitchonENUM_GunType (Variables|/Game/_Main/Blueprints/Guns/BP_Gun.BP_Gun_C|GetGunType _asbp_gun))
    (elif (> _commonammo 0)
      (bind _returnvalue (Game|SpawnActorfromClass "/Game/_Main/Blueprints/Guns/BP_Magazine.BP_Magazine_C" (Math|Transform|MakeTransform (Transformation|GetWorldLocation MotionController) "0, 0, 0" "1.000000,1.000000,1.000000") "Undefined" "MultiplyWithRoot" 0 0))
      (if (>= (Variables|/Game/_Main/Blueprints/Guns/BP_Magazine.BP_Magazine_C|GetRounds _returnvalue) _commonammo)
        ;[1 0.8906 0] FIX
        (Default|SetNewAmount _returnvalue (Variables|/Game/VRTemplate/Blueprints/VRPawn.VRPawn_C|GetCommonAmmo (Variables|Default|GetAs%20VRPawn))))
      (Default|TryGrabbingObject (Variables|Default|GetAs%20VRPawn) 0 (Variables|/Game/_Main/Blueprints/Guns/BP_Magazine.BP_Magazine_C|GetCurlGrabComponent _returnvalue) (Utilities|Enum|Equal(Enum) (Default|GetHeldbyHand (Variables|Default|GetGrabComponent)) "Right") true))))

(event EventBeginPlay
  (bind _asvrpawn (Utilities|Casting|CastToVRPawn (Game|GetPlayerCharacter 0)))
  (Variables|Default|SetAs%20VRPawn _asvrpawn))

(event Collision|EventActorBeginOverlap
  (params (OtherActor :type Actor%20Object%20Reference)))

(event EventTick
  (params (DeltaSeconds :type Float%20%28single-precision%29)))

(fn ConstructionScript)